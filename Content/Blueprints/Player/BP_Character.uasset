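; Player character Blueprint that handles pausing and the game-over state when an enemy catches the player.
; The Pause input lazily creates and caches a pause menu widget, then toggles it along with game pause, cursor visibility and input mode.
; Overlap of CaughtCapsule with an actor tagged Enemy runs once, disabling input, showing the game-over widget and cursor, and pausing the game.
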(event OnComponentBeginOverlap(CaughtCapsule)
  (params (OverlappedComponent :type Primitive%20Component%20Object%20Reference) (OtherActor :type Actor%20Object%20Reference) (OtherComp :type Primitive%20Component%20Object%20Reference) (OtherBodyIndex :type Integer) (bFromSweep :type Boolean) (SweepResult :type Hit%20Result%20Structure%20%28by%20ref%29))
  (bind _returnvalue (Game|GetPlayerController 0))
  (if (Actor|ActorHasTag OtherActor "Enemy")
    (Utilities|FlowControl|DoOnce false
      (:Completed
        (Input|DisableInput _returnvalue)
        (bind _returnvalue_2 (UserInterface|CreateWidget "/Game/HUD/Gameplay/GameOver_Widget.GameOver_Widget_C"))
        (UserInterface|Viewport|AddtoViewport _returnvalue_2 0)
        (Variables|/Script/Engine.PlayerController|SetbShowMouseCursor _returnvalue true)
        (Game|SetGamePaused true)))))

(event EventBeginPlay)

(event Collision|EventActorBeginOverlap
  (params (OtherActor :type Actor%20Object%20Reference)))

(event EventTick
  (params (DeltaSeconds :type Float%20%28single-precision%29)))

(event Input|ActionEvents|InputActionPause
  (params (Key :type Key%20Structure :default "None"))
  (bind _returnvalue (Game|GetPlayerController 0))
  (:Pressed
    (Utilities|IsValid (Variables|Default|GetPause%20Menu%20REF)
      (:Is%20Valid
        _)
      (:Is%20Not%20Valid
        (bind _returnvalue_2 (UserInterface|CreateWidget "/Game/HUD/Gameplay/PauseMenu_Widget.PauseMenu_Widget_C"))
        (Variables|Default|SetPause%20Menu%20REF _returnvalue_2)))
    (if (Game|IsGamePaused)
      (Widget|RemovefromParent (Variables|Default|GetPause%20Menu%20REF))
      (Game|SetGamePaused false)
      (Variables|/Script/Engine.PlayerController|SetbShowMouseCursor _returnvalue false)
      (Input|SetInputModeGameOnly _returnvalue)
      (else
        (UserInterface|Viewport|AddtoViewport (Variables|Default|GetPause%20Menu%20REF) 0)
        (Game|SetGamePaused true)
        (Variables|/Script/Engine.PlayerController|SetbShowMouseCursor _returnvalue true)
        (Input|SetInputModeGameandUI _returnvalue (Variables|Default|GetPause%20Menu%20REF) "DoNotLock" true)))))

(fn ConstructionScript)