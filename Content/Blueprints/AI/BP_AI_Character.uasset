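; AI character that draws a patrol view cone around its facing direction, clipped by blocking geometry.
; Construction derives the section count and angle step from the cone's angles; each Tick refreshes the origin and fans Visibility line traces across the arc.
; Adjacent hit points, or trace ends, form one procedural-mesh triangle per section, rebuilt every frame.
; The mesh is counter-rotated against the actor's facing because vertices use world-oriented offsets.
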(event EventBeginPlay)

(event Collision|EventActorBeginOverlap
  (params (OtherActor :type Actor%20Object%20Reference)))

(event EventTick
  (params (DeltaSeconds :type Float%20%28single-precision%29))
  (CallFunction|Update)
  (CallFunction|LineTracing))

(fn ConstructionScript
  (if (Variables|FieldOfVision|Debug|GetbRebuild)
    _
    (else
      _))
  (CallFunction|Start)
  (CallFunction|LineTracing))

(fn LineTracing
  (bind _startpoint (Variables|FieldOfVision|Auxiliary|GetStartPoint))
  (for _index (range 0 (Variables|FieldOfVision|Auxiliary|GetNumberOfSections))
    (LocalVariables|SetL_CurrentAngle (- (* _index (Variables|FieldOfVision|Auxiliary|GetdAngle)) (Variables|FieldOfVision|Base|GetHalfAngle)))
    (bind _outhit (Collision|LineTraceByChannel _startpoint (+ _startpoint (* (Math|Vector|RotateVectorAroundAxis (Transformation|GetActorForwardVector) (LocalVariables|GetL_CurrentAngle) "0, 0,1.000000") (Variables|FieldOfVision|Base|GetExternalRadius))) "TraceTypeQuery1" false 0 (Variables|FieldOfVision|Debug|GetDrawDebugType) true "(R=1.000000,G=0.000000,B=0.000000,A=1.000000)" "(R=0.000000,G=1.000000,B=0.000000,A=1.000000)" (Variables|FieldOfVision|Debug|GetDrawDebugTime)))
    (Utilities|Array|Add (Variables|Default|GetHitResult) _outhit))
  (CallFunction|CreateProceduralMesh))

(fn Start
  (Utilities|FlowControl|Sequence
    (:then_0
      (bind _output_get (Variables|FieldOfVision|Auxiliary|SetNumberOfSections (Math|Float|Ceil (/ (* (Variables|FieldOfVision|Base|GetHalfAngle) 2.0) (Variables|FieldOfVision|Base|GetDeltaAngle)))))
      (Variables|FieldOfVision|Auxiliary|SetdAngle (/ (* (Variables|FieldOfVision|Base|GetHalfAngle) 2.0) (Math|Conversions|ToFloat(Integer) _output_get))))
    (:then_1
      (Variables|FieldOfVision|Auxiliary|SetStartPoint (+ (Math|Vector|MakeVector 0.0 0.0 (- (Variables|FieldOfVision|Base|GetHeightOfCheck) 1e+02)) (Transformation|GetActorLocation))))
    (:then_2
      (Transformation|AddLocalOffset (Variables|Default|GetProceduralMesh) (Math|Vector|MakeVector 0.0 0.0 (- (Variables|FieldOfVision|Base|GetHeightOfShow) 1e+02)) false false))))

(fn CreateProceduralMesh
  (for _index (range 0 (- (Utilities|Array|LastIndex (Variables|Default|GetHitResult)) 1))
    (LocalVariables|SetI _index)
    (Utilities|FlowControl|Sequence
      (:then_0
        (if (.bBlockingHit (Collision|BreakHitResult (Utilities|Array|Get(acopy) (Variables|Default|GetHitResult) (LocalVariables|GetI))))
          (LocalVariables|SetL_LeftPoint (.Location (Collision|BreakHitResult (Utilities|Array|Get(acopy) (Variables|Default|GetHitResult) (LocalVariables|GetI)))))
          (else
            (LocalVariables|SetL_LeftPoint (.TraceEnd (Collision|BreakHitResult (Utilities|Array|Get(acopy) (Variables|Default|GetHitResult) (LocalVariables|GetI))))))))
      (:then_1
        (if (.bBlockingHit (Collision|BreakHitResult (Utilities|Array|Get(acopy) (Variables|Default|GetHitResult) (+ (LocalVariables|GetI) 1))))
          (LocalVariables|SetL_RightPoint (.Location (Collision|BreakHitResult (Utilities|Array|Get(acopy) (Variables|Default|GetHitResult) (+ (LocalVariables|GetI) 1)))))
          (else
            (LocalVariables|SetL_RightPoint (.TraceEnd (Collision|BreakHitResult (Utilities|Array|Get(acopy) (Variables|Default|GetHitResult) (+ (LocalVariables|GetI) 1))))))))
      (:then_2
        (Class|ProceduralMeshComponent|CreateMeshSectionLinearColor (Variables|Default|GetProceduralMesh) (LocalVariables|GetI) (Utilities|Array|MakeArray (- (Variables|FieldOfVision|Auxiliary|GetStartPoint) (Variables|FieldOfVision|Auxiliary|GetStartPoint)) (- (LocalVariables|GetL_LeftPoint) (Variables|FieldOfVision|Auxiliary|GetStartPoint)) (- (LocalVariables|GetL_RightPoint) (Variables|FieldOfVision|Auxiliary|GetStartPoint))) (Utilities|Array|MakeArray 0 2 1) 0 0 0 0 0 0 0 false)
        (Rendering|Material|SetMaterial (Variables|Default|GetProceduralMesh) (LocalVariables|GetI) "/Game/Assets/Materials/M_ViewConeAI_Patrol.M_ViewConeAI_Patrol"))))
  (Transformation|SetRelativeRotation (Variables|Default|GetProceduralMesh) (* (Math|Rotator|MakeRotfromX (Transformation|GetActorForwardVector)) -1) false false))

(fn Update
  (Variables|FieldOfVision|Auxiliary|SetStartPoint (+ (Math|Vector|MakeVector 0.0 0.0 (- (Variables|FieldOfVision|Base|GetHeightOfCheck) 1e+02)) (Transformation|GetActorLocation)))
  (Utilities|Array|Clear (Variables|Default|GetHitResult))
  (Class|ProceduralMeshComponent|ClearAllMeshSections (Variables|Default|GetProceduralMesh)))