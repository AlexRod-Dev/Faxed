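; AI controller for the patrol enemy that runs its behavior tree and reacts to perceiving the player.
; Perception updates broadcast sensed state and a curve-based detection speed, then set bIsAlert even on sight loss.
; The speed's distance input compares the stimulus location with itself, so it is always zero.
; SeenPlayer and LostPlayer swap the enemy's active material and set or clear TargetActor, with LostPlayer also clearing alert.
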(event OnTargetPerceptionUpdated(AIPerception)
  (params (Actor :type Actor%20Object%20Reference) (Stimulus :type AI%20Stimulus%20Structure))
  (bind (_age _expirationage _strength _stimuluslocation _receiverlocation _tag _bsuccessfullysensed) (Utilities|Struct|BreakAIStimulus Stimulus))
  (if (== Actor (Game|GetPlayerCharacter 0))
    (Default|CallSightRegisteredED _bsuccessfullysensed (Math|Curves|GetFloatValue (Variables|Default|GetSightCurve) (Math|Float|NormalizetoRange (Math|Vector|Distance(Vector) _stimuluslocation _stimuluslocation) 0.0 1e+03)))
    (AI|Components|Blackboard|SetValueasBool (Variables|Default|GetBlackboard) (Utilities|Name|MakeLiteralName "bIsAlert") true)))

(event Custom|SeenPlayer
  (bind _asbp_patrol_ai_enemy (Utilities|Casting|CastToBP_PatrolAI_Enemy (Game|GetInstigator)))
  (Variables|/Game/Blueprints/AI/BP_PatrolAI_Enemy.BP_PatrolAI_Enemy_C|SetActiveMaterial _asbp_patrol_ai_enemy (Variables|/Game/Blueprints/AI/BP_PatrolAI_Enemy.BP_PatrolAI_Enemy_C|GetAlertMaterial _asbp_patrol_ai_enemy))
  (AI|Components|Blackboard|SetValueasObject (Variables|Default|GetBlackboard) (Utilities|Name|MakeLiteralName "TargetActor") (Game|GetPlayerCharacter 0)))

(event Custom|Lost%20Player
  (bind _asbp_patrol_ai_enemy (Utilities|Casting|CastToBP_PatrolAI_Enemy (Game|GetInstigator)))
  (Variables|/Game/Blueprints/AI/BP_PatrolAI_Enemy.BP_PatrolAI_Enemy_C|SetActiveMaterial _asbp_patrol_ai_enemy (Variables|/Game/Blueprints/AI/BP_PatrolAI_Enemy.BP_PatrolAI_Enemy_C|GetPatrolMaterial _asbp_patrol_ai_enemy))
  (AI|Components|Blackboard|SetValueasObject (Variables|Default|GetBlackboard) (Utilities|Name|MakeLiteralName "TargetActor") 0)
  (AI|Components|Blackboard|SetValueasBool (Variables|Default|GetBlackboard) (Utilities|Name|MakeLiteralName "bIsAlert") false))

(event EventBeginPlay
  (Utilities|Casting|CastToBP_PatrolAI_Enemy (Game|GetInstigator))
  (AI|RunBehaviorTree "/Game/Blueprints/AI/PatrolEnemyBT.PatrolEnemyBT")
  (bind _asbp_patrol_ai_enemy (Utilities|Casting|CastToBP_PatrolAI_Enemy (Pawn|GetControlledPawn)))
  (Variables|Default|SetAs%20BP%20Patrol%20AI%20Enemy _asbp_patrol_ai_enemy))

(event EventTick
  (params (DeltaSeconds :type Float%20%28single-precision%29)))

(fn ConstructionScript)