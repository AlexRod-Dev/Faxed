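; AI character Blueprint that draws its field of view as a flat procedural-mesh cone.
; Each tick it runs the VisionCone EQS query and, when finished, converts the result locations into actor-relative vertices with Z flattened.
; It builds fan triangle indices around vertex 0, then recreates the mesh section with the patrol material.
; The mesh's world rotation is zeroed to match the world-axis offsets.
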(event Custom|MakeCone
  (params (QueryInstance :type Env%20Query%20Instance%20Blueprint%20Wrapper%20Object%20Reference) (QueryStatus :type EEnvQueryStatus%20Enum :default "Processing"))
  (bind _resultlocations (AI|EQS|GetQueryResultsasLocations QueryInstance))
  (bind _output_get (Variables|Default|SetSightPoints _resultlocations))
  (bind (_vertices _triangles) (CallFunction|ConvertSightPointstoVertices _output_get))
  (CallFunction|MaketheCone _vertices _triangles))

(event EventBeginPlay
  (Utilities|Array|Resize (Variables|Default|GetVertices) 50))

(event Collision|EventActorBeginOverlap
  (params (OtherActor :type Actor%20Object%20Reference)))

(event EventTick
  (params (DeltaSeconds :type Float%20%28single-precision%29))
  (bind _returnvalue (AI|EQS|RunEQSQuery "/Game/Blueprints/AI/VisionCone/VisionCone.VisionCone" self "AllMatching"))
  (EventDispatchers|BindEventtoOnQueryFinishedEvent _returnvalue (delegate Custom|MakeCone)))

(fn ConstructionScript)

(fn ConvertSightPointstoVertices
  (params (SightPoints :type Array%20of%20Vectors))
  (bind _returnvalue (Transformation|GetActorLocation))
  (bind _vertices (Variables|Default|GetVertices))
  (bind _returnvalue_2 (Utilities|Array|Length _vertices))
  (bind (_x _y) (Math|Vector|BreakVector _returnvalue))
  (bind _returnvalue_3 (* _returnvalue_2 3))
  (Utilities|Array|SetArrayElem :TargetArray (Variables|Default|GetVertices))
  (for (_array_element _array_index) SightPoints
    (Utilities|Array|SetArrayElem (Variables|Default|GetVertices) _array_index (Math|Vector|MakeVector (- (.X (Math|Vector|BreakVector _array_element)) _x) (- (.Y (Math|Vector|BreakVector _array_element)) _y) 0.0)))
  (Utilities|Array|Resize (Variables|Default|GetTriangles) _returnvalue_3)
  (for _index (range 0 _returnvalue_3)
    (Utilities|Array|SetArrayElem (Variables|Default|GetTriangles) (* _index 3) 0)
    (Utilities|Array|SetArrayElem (Variables|Default|GetTriangles) (+ (* _index 3) 1) (+ _index 1))
    (Utilities|Array|SetArrayElem (Variables|Default|GetTriangles) (+ (+ (* _index 3) 1) 1) (+ (+ _index 1) 1)))
  (return (Variables|Default|GetVertices) (Variables|Default|GetTriangles)))

(fn MaketheCone
  (params (Vertice :type Array%20of%20Vectors) (Triangles :type Array%20of%20Integers))
  (bind _visioncone (Variables|Default|GetVisionCone))
  (Class|ProceduralMeshComponent|CreateMeshSectionLinearColor _visioncone 0 Vertice Triangles 0 0 0 0 0 0 0 false)
  (Rendering|Material|SetMaterial _visioncone 0 "/Game/Assets/Materials/ViewConeAI_Patrol_Mat.ViewConeAI_Patrol_Mat")
  (Transformation|SetWorldRotation _visioncone "0, 0, 0" false false))