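; AI controller for BP_StaticAI_Enemy, a stationary enemy that watches for the player with an intermittent sight cone.
; BeginPlay runs StaticEnemyBT and starts a looping timer that FlipFlops the cone and sight sense on and off.
; Perception updates on the player report detection with the enemy's DetectionSpeed and write alert state and location to the Blackboard.
; SeenPlayer and LostPlayer swap alert or patrol materials and set or clear TargetActor.
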(event OnTargetPerceptionUpdated(AIPerception)
  (params (Actor :type Actor%20Object%20Reference) (Stimulus :type AI%20Stimulus%20Structure))
  (bind (_age _expirationage _strength _stimuluslocation _receiverlocation _tag _bsuccessfullysensed) (Utilities|Struct|BreakAIStimulus Stimulus))
  (if (== Actor (Game|GetPlayerCharacter 0))
    (Default|CallSightRegisteredED _bsuccessfullysensed (Variables|/Game/Blueprints/AI/BP_StaticAI_Enemy.BP_StaticAI_Enemy_C|GetDetection%20Speed (stale EventBeginPlay _asbp_static_ai_enemy)))
    (AI|Components|Blackboard|SetValueasVector (Variables|Default|GetBlackboard) (Utilities|Name|MakeLiteralName "TargetLocation") _stimuluslocation)
    (AI|Components|Blackboard|SetValueasBool (Variables|Default|GetBlackboard) (Utilities|Name|MakeLiteralName "bIsAlert") true)))

(event Custom|ConeVisibility
  (bind _returnvalue (Game|GetInstigator))
  (bind _aiperception (Variables|Default|GetAIPerception))
  (Utilities|FlowControl|FlipFlop
    (:A
      (bind _asbp_static_ai_enemy (Utilities|Casting|CastToBP_StaticAI_Enemy _returnvalue))
      (Variables|/Game/Blueprints/AI/BP_StaticAI_Enemy.BP_StaticAI_Enemy_C|SetbActiveCone _asbp_static_ai_enemy true)
      (Class|AIPerceptionComponent|SetSenseEnabled _aiperception "/Script/AIModule.AISense_Sight" true))
    (:B
      (bind _asbp_static_ai_enemy_2 (Utilities|Casting|CastToBP_StaticAI_Enemy _returnvalue))
      (Variables|/Game/Blueprints/AI/BP_StaticAI_Enemy.BP_StaticAI_Enemy_C|SetbActiveCone _asbp_static_ai_enemy_2 false)
      (Class|AIPerceptionComponent|SetSenseEnabled _aiperception "/Script/AIModule.AISense_Sight" false))))

(event Custom|SeenPlayer
  (bind _asbp_static_ai_enemy (Utilities|Casting|CastToBP_StaticAI_Enemy (Game|GetInstigator)))
  (Variables|/Game/Blueprints/AI/BP_StaticAI_Enemy.BP_StaticAI_Enemy_C|SetActiveMaterial _asbp_static_ai_enemy (Variables|/Game/Blueprints/AI/BP_StaticAI_Enemy.BP_StaticAI_Enemy_C|GetAlertMaterial _asbp_static_ai_enemy))
  (AI|Components|Blackboard|SetValueasObject (Variables|Default|GetBlackboard) (Utilities|Name|MakeLiteralName "TargetActor") (Game|GetPlayerCharacter 0)))

(event Custom|Lost%20Player
  (bind _asbp_static_ai_enemy (Utilities|Casting|CastToBP_StaticAI_Enemy (Game|GetInstigator)))
  (Variables|/Game/Blueprints/AI/BP_StaticAI_Enemy.BP_StaticAI_Enemy_C|SetActiveMaterial _asbp_static_ai_enemy (Variables|/Game/Blueprints/AI/BP_StaticAI_Enemy.BP_StaticAI_Enemy_C|GetPatrolMaterial _asbp_static_ai_enemy))
  (AI|Components|Blackboard|SetValueasObject (Variables|Default|GetBlackboard) (Utilities|Name|MakeLiteralName "TargetActor") 0)
  (AI|Components|Blackboard|SetValueasBool (Variables|Default|GetBlackboard) (Utilities|Name|MakeLiteralName "bIsAlert") false))

(event EventBeginPlay
  (bind _asbp_static_ai_enemy (Utilities|Casting|CastToBP_StaticAI_Enemy (Game|GetInstigator)))
  (Utilities|Time|SetTimerbyEvent (delegate Custom|ConeVisibility) (Variables|/Game/Blueprints/AI/BP_StaticAI_Enemy.BP_StaticAI_Enemy_C|GetCone%20timer _asbp_static_ai_enemy) true -3.0)
  (AI|RunBehaviorTree "/Game/Blueprints/AI/StaticEnemyBT.StaticEnemyBT")
  (bind _asbp_static_ai_enemy_2 (Utilities|Casting|CastToBP_StaticAI_Enemy (Pawn|GetControlledPawn)))
  (Variables|Default|SetAs%20BP%20Static%20AI%20Enemy _asbp_static_ai_enemy_2))

(event EventTick
  (params (DeltaSeconds :type Float%20%28single-precision%29)))

(fn ConstructionScript)