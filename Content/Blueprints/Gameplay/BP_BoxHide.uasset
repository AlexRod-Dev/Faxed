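; BP_BoxHide is a hiding spot that the player enters and leaves with Interact.
; InteractArea overlap with BP_Character enables input and opens a gate; leaving reverses both.
; ToggleHide switches player visibility and collision and blends the camera between box and player, then input and gate are re-enabled after a short delay.
; Hiding also clears the target and alert state on the first BP_PatrolAI_Controller found.
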(event OnComponentBeginOverlap(InteractArea)
  (params (OverlappedComponent :type Primitive%20Component%20Object%20Reference) (OtherActor :type Actor%20Object%20Reference) (OtherComp :type Primitive%20Component%20Object%20Reference) (OtherBodyIndex :type Integer) (bFromSweep :type Boolean) (SweepResult :type Hit%20Result%20Structure%20%28by%20ref%29))
  (bind _asbp_character (Utilities|Casting|CastToBP_Character OtherActor))
  (Variables|Default|SetPlayer%20Ref _asbp_character)
  (Input|EnableInput (Game|GetPlayerController 0))
  (Utilities|FlowControl|Gate true) ; enters at Open
)

(event OnComponentEndOverlap(InteractArea)
  (params (OverlappedComponent :type Primitive%20Component%20Object%20Reference) (OtherActor :type Actor%20Object%20Reference) (OtherComp :type Primitive%20Component%20Object%20Reference) (OtherBodyIndex :type Integer))
  (bind _returnvalue (Game|GetPlayerController 0))
  (Utilities|Casting|CastToBP_Character OtherActor)
  (Input|DisableInput _returnvalue)
  (Utilities|FlowControl|Gate true) ; enters at Close
)

(event EventBeginPlay)

(event Collision|EventActorBeginOverlap
  (params (OtherActor :type Actor%20Object%20Reference)))

(event EventTick
  (params (DeltaSeconds :type Float%20%28single-precision%29)))

(event Input|ActionEvents|InputActionInteract
  (params (Key :type Key%20Structure))
  (:Pressed
    (Utilities|FlowControl|Gate true :!label _label
      (:Exit
        (Utilities|FlowControl|Sequence
          (:then_0
            (CallFunction|ToggleHide)
            (Utilities|FlowControl|Delay 0.2)
            (Input|EnableInput (Game|GetPlayerController 0))
            (goto _label Open)))))))

(fn ConstructionScript)

(fn ToggleHide
  (bind _returnvalue (Game|GetPlayerController 0))
  (bind _player_ref (Variables|Default|GetPlayer%20Ref))
  (if (Variables|Default|GetbIsHiding)
    (Variables|Default|SetbIsHiding false)
    (Rendering|SetActorHiddenInGame _player_ref false)
    (Collision|SetActorEnableCollision _player_ref true)
    (Game|Player|SetViewTargetwithBlend _returnvalue _player_ref 0.3 "VTBlend_Linear" 0.0 false)
    (else
      (Variables|Default|SetbIsHiding true)
      (Rendering|SetActorHiddenInGame _player_ref true)
      (Collision|SetActorEnableCollision _player_ref false)
      (Game|Player|SetViewTargetwithBlend _returnvalue self 0.3 "VTBlend_Linear" 0.0 false)
      (bind _returnvalue_2 (Actor|GetActorOfClass "/Game/Blueprints/AI/BP_PatrolAI_Controller.BP_PatrolAI_Controller_C"))
      (AI|Components|Blackboard|SetValueasObject (Variables|/Script/AIModule.AIController|GetBlackboard _returnvalue_2) (Utilities|Name|MakeLiteralName "TargetActor") 0)
      (AI|Components|Blackboard|SetValueasBool (Variables|/Script/AIModule.AIController|GetBlackboard _returnvalue_2) (Utilities|Name|MakeLiteralName "bIsAlert") false))))