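; BP_NextLevel is a level-exit trigger that shows an end-of-level screen when any actor overlaps it.
; On overlap it switches on the current level name, creating NextLevel_Widget for Level 1 and Level 2 and EndGame_Widget for Level 3.
; Either widget is added to the viewport, then the game pauses, the mouse cursor appears and input switches to Game and UI mode.
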(event EventBeginPlay)

(event Collision|EventActorBeginOverlap
  (params (OtherActor :type Actor%20Object%20Reference))
  (bind _returnvalue (Game|GetPlayerController 0))
  (bind _returnvalue_2 (Game|GetCurrentLevelName true))
  (switch string _returnvalue_2
    (:Level1
      (bind _returnvalue_3 (UserInterface|CreateWidget "/Game/HUD/Gameplay/NextLevel_Widget.NextLevel_Widget_C" :!label _label))
      (UserInterface|Viewport|AddtoViewport _returnvalue_3 0)
      (Variables|/Script/Engine.PlayerController|SetbShowMouseCursor _returnvalue true)
      (Game|SetGamePaused true)
      (Input|SetInputModeGameandUI _returnvalue 0 "DoNotLock" true))
    (:Level2
      (goto _label))
    (:Level3
      (bind _returnvalue_4 (UserInterface|CreateWidget "/Game/HUD/Gameplay/EndGame_Widget.EndGame_Widget_C"))
      (UserInterface|Viewport|AddtoViewport _returnvalue_4 0)
      (Variables|/Script/Engine.PlayerController|SetbShowMouseCursor _returnvalue true)
      (Game|SetGamePaused true)
      (Input|SetInputModeGameandUI _returnvalue 0 "DoNotLock" true))))

(event EventTick
  (params (DeltaSeconds :type Float%20%28single-precision%29)))

(fn ConstructionScript)